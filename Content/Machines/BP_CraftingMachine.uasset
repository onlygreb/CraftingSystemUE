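; Crafting machine actor that connects to the player's HUD to show an open-machine prompt and the crafting panel.
; On BeginPlay it registers its overlap box, caches player 0's BP_UI HUD and stores the arrow's location as the item spawn point.
; Its events forward prompt visibility, recipe IDs and nearby item IDs to the HUD, passing itself to the panel.
; Overlap detection and crafting logic are not in these graphs.
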(event `self.ReceiveBeginPlay`
  (set `self.OverlapComponent` (`self.OverlapBox`))
  (bind _asbp_ui (cast `/Game/Widgets/BP_UI` (`PlayerController.GetHUD` (`GameplayStatics.GetPlayerController` 0))))
  (set `self.BP_UI` _asbp_ui)
  (set `self.locationToSpawnItems` (`SceneComponent.K2_GetComponentLocation` (`self.Arrow`))))

(event `self.ToggleShowOpenMachineText`
  (params (show :type Boolean))
  (`/Game/Widgets/BP_UI.ToggleOpenCraftingMachineText` (`self.BP_UI`) show))

(event `self.OnOpenMachine`
  (params (recipesIDArray :type "Array of Integer (by ref)") (currentItemsInProximityID :type "Array of Integer (by ref)"))
  (`/Game/Widgets/BP_UI.OpenCraftingMachinePanel` (`self.BP_UI`) recipesIDArray currentItemsInProximityID self))

(fn `UserConstructionScript`)