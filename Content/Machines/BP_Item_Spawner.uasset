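; BP_Item_Spawner is a machine that spawns a configured item when a non-item actor enters its trigger box.
; It looks up ItemIDToSpawn in DT_Items and spawns that row's item actor at the Arrow's location.
; A HasSpawned flag blocks repeat spawns until a non-item actor leaves the box and a short delay passes.
; A failed cast to CT_Item filters both overlap events, so items cannot trigger or reset it.
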(event `self.Box.OnComponentBeginOverlap`
  (params (OverlappedComponent :type "PrimitiveComponent Object Reference") (OtherActor :type "Actor Object Reference") (OtherComp :type "PrimitiveComponent Object Reference") (OtherBodyIndex :type Integer) (bFromSweep :type Boolean) (SweepResult :type "HitResult Structure (by ref)"))
  (cast `CT_Item` OtherActor
    (:`CastFailed`
      (if (== (`self.hasSpawned`) false)
        (bind _returnvalue (`|GetDataTableRow` "/Game/DataTables/DT_Items.DT_Items" (`KismetStringLibrary.Conv_StringToName` (`KismetStringLibrary.Conv_Int64ToString` (`self.ItemIDToSpawn`))))
          (:`then`
            (`self.SpawnItem` (`.ItemActor_16_0553A43E44CE50C39945279B3B818F4B` (break `/Game/DataTables/ST_Item` _returnvalue)) (`SceneComponent.K2_GetComponentLocation` (`self.Arrow`)))
            (set `self.hasSpawned` true)))))))

(event `self.Box.OnComponentEndOverlap`
  (params (OverlappedComponent :type "PrimitiveComponent Object Reference") (OtherActor :type "Actor Object Reference") (OtherComp :type "PrimitiveComponent Object Reference") (OtherBodyIndex :type Integer))
  (cast `CT_Item` OtherActor
    (:`CastFailed`
      (`KismetSystemLibrary.Delay` 0.3)
      (set `self.hasSpawned` false))))

(fn `UserConstructionScript`)